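; BP_Enemy is an enemy character with walk and sprint movement and a simple line-of-sight check for the player.
; BeginPlay applies walk speed, while BeginSprint and EndSprint switch the movement speed and set IsSprint.
; CanSeePlayerPawn traces forward from the actor up to SightRange, with debug drawing, and tests the hit actor for the Player tag.
; The event graph leaves that check unwired and calls neither sprint function.
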(event EventBeginPlay
  (Variables|/Script/Engine.CharacterMovementComponent|SetMaxWalkSpeed (Variables|Character|GetCharacterMovement) (Variables|Default|GetWalkSpeed)))

(event Collision|EventActorBeginOverlap
  (params (OtherActor :type Actor%20Object%20Reference)))

(event EventTick
  (params (DeltaSeconds :type Float%20%28single-precision%29)))

(fn ConstructionScript)

(fn BeginSprint
  (Variables|/Script/Engine.CharacterMovementComponent|SetMaxWalkSpeed (Variables|Character|GetCharacterMovement) (Variables|Default|GetSprintSpeed))
  (Variables|Default|SetisSprint true))

(fn EndSprint
  (Variables|/Script/Engine.CharacterMovementComponent|SetMaxWalkSpeed (Variables|Character|GetCharacterMovement) (Variables|Default|GetWalkSpeed))
  (Variables|Default|SetisSprint false))

(fn CanSeePlayerPawn
  (bind _returnvalue (Transformation|GetActorLocation))
  (bind (_outhit _returnvalue_2) (Collision|LineTraceByChannel _returnvalue (+ _returnvalue (* (Math|Vector|GetForwardVector (Variables|Collision|GetCapsuleComponent)) (Variables|Default|GetSightRange))) "TraceTypeQuery3" false 0 "ForOneFrame"))
  (if _returnvalue_2
    (return (Actor|ActorHasTag (.HitActor (Collision|BreakHitResult _outhit)) "Player"))))